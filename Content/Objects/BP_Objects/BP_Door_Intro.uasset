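; BP_Door_Intro is an intro door that springs a scripted attack by the neighbor character (Sosed).
; On BeginPlay it finds and caches the BP_Sosed and puts it in the TUTORIAL state.
; When a BP_Human enters its Box trigger, it teleports Sosed to the NeighborTransform location and switches it to ATTACK.
; The construction script applies the configured mesh rotation, and only DoorMesh counts as the action component.
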(event `self.Box.OnComponentBeginOverlap`
  (params (OverlappedComponent :type "PrimitiveComponent Object Reference") (OtherActor :type "Actor Object Reference") (OtherComp :type "PrimitiveComponent Object Reference") (OtherBodyIndex :type Integer) (bFromSweep :type Boolean) (SweepResult :type "HitResult Structure (by ref)"))
  (bind _sosed (`self.Sosed`))
  (cast `/Game/Player/BP_Human` OtherActor)
  (`self.K2_SetActorLocation` _sosed (`SceneComponent.K2_GetComponentLocation` (`self.NeighborTransform`)) false true)
  (`Sosed.SetState` _sosed "NS_ATTACK"))

(event `self.ReceiveBeginPlay`
  (bind _returnvalue (`Sosed.FindSosed`))
  (bind _asbp_sosed (cast `/Game/Sosed/BP_Sosed` _returnvalue))
  (bind _output_get (set `self.Sosed` _asbp_sosed))
  (`Sosed.SetState` _output_get "NS_TUTORIAL"))

(fn `OnIsActionComponent`
  (params (Component :type "PrimitiveComponent Object Reference"))
  (returns (Result :type Boolean))
  (return (== Component (`self.DoorMesh`))))

(fn `UserConstructionScript`
  (`SceneComponent.K2_SetRelativeRotation` (`self.DoorMesh`) (`self.DoorMeshRotation`) false false))