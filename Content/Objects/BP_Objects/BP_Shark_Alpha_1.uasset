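; BP_Shark_Alpha_1 is a shark object that reacts to changes between Swim and Freeze states.
; Swim restarts the Fan's rotation from the beginning and activates the swim and pool sound cues, while Freeze deactivates both cues.
; Both states set the FlatComponent to Movable.
; The Fan stop call is disconnected, so Freeze leaves the rotation state untouched.
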(event `self.OnChangeSharkState`
  (params (NewState :type "ESharkState Enum" :default "Free"))
  (bind _flatcomponent (`self.FlatComponent`))
  (bind _shark_swim_cue (`self.shark_swim_Cue`))
  (switch `ESharkState` NewState
    (:`Swim`
      (`FlatComponent.SetFlatType` _flatcomponent "FT_Movable")
      (`RotationComponent.SetRotationState` (`self.Fan`) "RotationFromBegin")
      (`ActorComponent.Activate` _shark_swim_cue false)
      (`ActorComponent.Activate` (`self.shark_pool_Cue`) false))
    (:`Freeze`
      (`FlatComponent.SetFlatType` _flatcomponent "FT_Movable")
      (`ActorComponent.Deactivate` _shark_swim_cue)
      (`ActorComponent.Deactivate` (`self.shark_pool_Cue`)))))

(fn `UserConstructionScript`
  (`parent.UserConstructionScript`))