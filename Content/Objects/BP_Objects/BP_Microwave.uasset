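; BP_Microwave is an interactive microwave object with a door that players can open and close.
; An action on the Door component toggles its moving state, so triggering it mid-motion reverses the door's direction.
; The door's state-change event plays the matching open or close sound cue when movement starts.
; Every component reports itself as an action component, though only the Door responds.
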(event `self.OnEventAction`
  (params (ActionMaker :type "Actor Object Reference") (SpecialComponent :type "PrimitiveComponent Object Reference"))
  (bind _door (`self.Door`))
  (bind _door_2 (`self.Door`))
  (if (== SpecialComponent _door)
    (switch `EMovingState` (`MovingComponent.GetMovingState` _door)
      (:`MS_OPEN`
        (`MovingComponent.SetMovingState` _door_2 "MS_CLOSING" :!label _label))
      (:`MS_CLOSE`
        (`MovingComponent.SetMovingState` _door_2 "MS_OPENING" :!label _label_2))
      (:`MS_OPENING`
        (goto _label))
      (:`MS_CLOSING`
        (goto _label_2)))))

(event `self.Door.OnChangeMovingState`
  (params (NewState :type "EMovingState Enum" :default "MS_OPEN"))
  (switch `EMovingState` NewState
    (:`MS_OPENING`
      (`AudioComponent.Play` (`self.microwave_open_door_Cue`) 0.0))
    (:`MS_CLOSING`
      (`AudioComponent.Play` (`self.microwave_close_door_Cue`) 0.0))))

(fn `OnIsActionComponent`
  (params (Component :type "PrimitiveComponent Object Reference"))
  (returns (Result :type Boolean))
  (return true))

(fn `UserConstructionScript`)